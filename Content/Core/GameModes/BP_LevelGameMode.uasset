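; BP_LevelGameMode is a level game mode that shows the HUD, times the level and scores it from time and pins knocked.
; Tick adds delta seconds to Time only while TimerIsRunning is false, despite the Start/Stop event names, then updates the HUD.
; EndLevel waits through a delay, passes Time, MaxTime and PinsKnocked to CalculateScore, and only prints the results.
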(event Custom|TimerTick
  (if (not (Variables|Default|GettimerIsRunning))
    (bind _output_get (Variables|Default|Settime (+ (Variables|Default|Gettime) (Utilities|Time|GetWorldDeltaSeconds))))))

(event Custom|EndLevel
  (bind _pinsknocked (Variables|Default|GetPinsKnocked))
  (bind _time (Variables|Default|Gettime))
  (Utilities|FlowControl|Delay 5.0)
  (bind _returnvalue (Class|ScoringAPI|CalculateScore _time (Variables|Default|GetmaxTime) _pinsknocked))
  (Development|PrintString (Utilities|String|ToString(Integer) _returnvalue))
  (Development|PrintString (Utilities|String|ToString(Float) _time))
  (Development|PrintString (Utilities|String|ToString(Integer) _pinsknocked)))

(event Custom|StartTimer
  (Variables|Default|SettimerIsRunning true))

(event Custom|ResetTimer
  (Variables|Default|Settime 0.0))

(event Custom|StopTimer
  (Variables|Default|SettimerIsRunning false))

(event EventBeginPlay
  ;[1 1 1] Display HUD and create HUD ref
  (bind _returnvalue (UserInterface|CreateWidget "/Game/UI/GameHUDUI.GameHUDUI_C"))
  (Variables|Default|SetGameHUD _returnvalue)
  (UserInterface|Viewport|AddtoViewport (Variables|Default|GetGameHUD) 0))

(event EventTick
  (params (DeltaSeconds :type Float%20%28single-precision%29))
  (CallFunction|TimerTick)
  ;[1 1 1] Update Time in HUD
  (Default|UpdateTime (Variables|Default|GetGameHUD) (Variables|Default|Gettime)))

(fn ConstructionScript)