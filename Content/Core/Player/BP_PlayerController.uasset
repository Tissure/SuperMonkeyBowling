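; BP_PlayerController is the player controller that drives a rolling-sphere BP_PlayerPawn through Enhanced Input.
; On BeginPlay it caches the pawn and adds the IMC_Gameplay mapping context.
; Look actions feed controller yaw and pitch.
; Move input applies an angular impulse to the pawn's Sphere around the negated camera-yaw forward vector, scaled by RotationSpeed and input, as a mass-independent velocity change.
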(event Input|EnhancedActionEvents|EnhancedInputActionIA_Move
  (params (ActionValue :type Float%20%28double-precision%29) (ElapsedSeconds :type Float%20%28double-precision%29) (TriggeredSeconds :type Float%20%28double-precision%29) (InputAction :type Input%20Action%20Object%20Reference :default "/Game/Core/Input/IA_Move.IA_Move"))
  ;[1 1 1] Movement
  (Class|PrimitiveComponent|AddAngularImpulseinDegrees (Variables|/Game/Core/Player/BP_PlayerPawn.BP_PlayerPawn_C|GetSphere (stale EventBeginPlay _asbp_player_pawn)) (Math|Vector|NegateVector (* (Math|Vector|GetForwardVector (Math|Rotator|MakeRotator 0.0 0.0 (.yaw (Pawn|GetControlRotation :!class /Script/Engine.Controller)))) (* (Variables|/Game/Core/Player/BP_PlayerPawn.BP_PlayerPawn_C|GetRotation%20Speed (stale EventBeginPlay _asbp_player_pawn)) ActionValue))) "None" true))

(event Input|EnhancedActionEvents|EnhancedInputActionIA_LookLeftRight
  (params (ActionValue :type Float%20%28double-precision%29) (ElapsedSeconds :type Float%20%28double-precision%29) (TriggeredSeconds :type Float%20%28double-precision%29) (InputAction :type Input%20Action%20Object%20Reference :default "/Game/Core/Input/IA_LookLeftRight.IA_LookLeftRight"))
  (Pawn|Input|AddControllerYawInput (stale EventBeginPlay _asbp_player_pawn) ActionValue))

(event Input|EnhancedActionEvents|EnhancedInputActionIA_LookUpDown
  (params (ActionValue :type Float%20%28double-precision%29) (ElapsedSeconds :type Float%20%28double-precision%29) (TriggeredSeconds :type Float%20%28double-precision%29) (InputAction :type Input%20Action%20Object%20Reference :default "/Game/Core/Input/IA_LookUpDown.IA_LookUpDown"))
  (Pawn|Input|AddControllerPitchInput (stale EventBeginPlay _asbp_player_pawn) ActionValue))

(event EventBeginPlay
  (bind _asbp_player_pawn (Utilities|Casting|CastToBP_PlayerPawn (Game|Player|GetPlayerPawn 0)))
  (bind _asplayer_controller (Utilities|Casting|CastToPlayerController (Pawn|GetController _asbp_player_pawn)))
  (Utilities|IsValid (PlayerController|LocalPlayerSubsystems|GetEnhancedInputLocalPlayerSubsystem _asplayer_controller)
    (:Is%20Valid
      (Input|AddMappingContext (PlayerController|LocalPlayerSubsystems|GetEnhancedInputLocalPlayerSubsystem _asplayer_controller) "/Game/Core/Input/IMC_Gameplay.IMC_Gameplay" 0 "(bIgnoreAllPressedKeysUntilRelease=True,bForceImmediately=False,bNotifyUserSettings=False)"))))

(event EventTick
  (params (DeltaSeconds :type Float%20%28single-precision%29)))

(fn ConstructionScript)