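; Player pawn that moves as a physics-rolled sphere, with Enhanced Input set up on possession.
; Look inputs drive controller yaw and pitch, while move input applies an angular impulse around the negated yaw-only forward axis, scaled by RotationSpeed, for sideways roll.
; The pause input opens the pause widget, shows the cursor and pauses the game.
; Tick logs velocity, and a leftover AddMovementInput node is unconnected.
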(event Input|EnhancedActionEvents|EnhancedInputActionIA_Move
  (params (ActionValue :type Float%20%28double-precision%29) (ElapsedSeconds :type Float%20%28double-precision%29) (TriggeredSeconds :type Float%20%28double-precision%29) (InputAction :type Input%20Action%20Object%20Reference :default "/Game/Core/Input/IA_Move.IA_Move"))
  ;[1 1 1] Movement
  (Class|PrimitiveComponent|AddAngularImpulseinDegrees (Variables|Default|GetSphere) (Math|Vector|NegateVector (* (Math|Vector|GetForwardVector (Math|Rotator|MakeRotator 0.0 0.0 (.yaw (Pawn|GetControlRotation :!class /Script/Engine.Pawn)))) (* (Variables|Default|GetRotation%20Speed) ActionValue))) "None" true))

(event Input|EnhancedActionEvents|EnhancedInputActionIA_LookLeftRight
  (params (ActionValue :type Float%20%28double-precision%29) (ElapsedSeconds :type Float%20%28double-precision%29) (TriggeredSeconds :type Float%20%28double-precision%29) (InputAction :type Input%20Action%20Object%20Reference :default "/Game/Core/Input/IA_LookLeftRight.IA_LookLeftRight"))
  (Pawn|Input|AddControllerYawInput ActionValue))

(event Input|EnhancedActionEvents|EnhancedInputActionIA_LookUpDown
  (params (ActionValue :type Float%20%28double-precision%29) (ElapsedSeconds :type Float%20%28double-precision%29) (TriggeredSeconds :type Float%20%28double-precision%29) (InputAction :type Input%20Action%20Object%20Reference :default "/Game/Core/Input/IA_LookUpDown.IA_LookUpDown"))
  (Pawn|Input|AddControllerPitchInput ActionValue))

(event Input|EnhancedActionEvents|EnhancedInputActionIA_PauseGame
  (params (ActionValue :type Boolean) (ElapsedSeconds :type Float%20%28double-precision%29) (TriggeredSeconds :type Float%20%28double-precision%29) (InputAction :type Input%20Action%20Object%20Reference :default "/Game/Core/Input/IA_PauseGame.IA_PauseGame"))
  (bind _returnvalue (Game|GetPlayerController 0))
  ;[1 1 1] Open Pause menu
  (:Started
    (bind _returnvalue_2 (UserInterface|CreateWidget "/Game/UI/PauseUI.PauseUI_C"))
    (UserInterface|Viewport|AddtoViewport _returnvalue_2 0)
    (Variables|/Script/Engine.PlayerController|SetbShowMouseCursor _returnvalue true)
    (Input|SetInputModeUIOnly _returnvalue 0 "DoNotLock" false)
    (Game|SetGamePaused true)))

(event EventPossessed
  (params (NewController :type Controller%20Object%20Reference))
  (bind _asplayer_controller (Utilities|Casting|CastToPlayerController NewController))
  (Input|EnableInput _asplayer_controller)
  (Utilities|IsValid (PlayerController|LocalPlayerSubsystems|GetEnhancedInputLocalPlayerSubsystem _asplayer_controller)
    (:Is%20Valid
      (Input|AddMappingContext (PlayerController|LocalPlayerSubsystems|GetEnhancedInputLocalPlayerSubsystem _asplayer_controller) "/Game/Core/Input/IMC_Gameplay.IMC_Gameplay" 0 "(bIgnoreAllPressedKeysUntilRelease=True,bForceImmediately=False,bNotifyUserSettings=False)"))))

(event EventTick
  (params (DeltaSeconds :type Float%20%28single-precision%29))
  (Utilities|String|LogString (Utilities|String|ToString(Vector) (Transformation|GetVelocity))))

(fn ConstructionScript)